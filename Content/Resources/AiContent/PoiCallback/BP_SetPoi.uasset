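; BP_SetPoi is a point-of-interest callback that switches the AI controller's current point of interest to the configured PoiIndex.
; An optional DontSetAfterClockEnd flag skips the switch when a POI_ClockAndPosition was completed by its clock.
; It logs an error if the index does not exist or if the flag is used on another point-of-interest type.
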(event `self.Execute`
  (params (PointOfInterest :type "AiPointOfInterest Object Reference"))
  (if (`self.DontSetAfterClockEnd`)
    (bind _aspoi_clock_and_position (cast `POI_ClockAndPosition` PointOfInterest)
      (:`then`
        (if (not (`POI_ClockAndPosition.IsCompleteCausedByClock` _aspoi_clock_and_position))
          (bind _returnvalue (`VillagerAiController.SetCurrentPointOfInterest` (`AiPointOfInterest.GetAiController` PointOfInterest) (`self.PoiIndex`) :!label _label))
          (`Log.Error_WithCondition` "Poi Index dont exists" (not _returnvalue) "LO_Both")))
      (:`CastFailed`
        (`Log.Error` "\"DontSetAfterClockEnd\" cant be used only with ClockAndPosition and only after Complete" "LO_Both")))
    (else
      (goto _label))))