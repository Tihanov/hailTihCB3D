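; BP_Spawner is a utility Blueprint that spawns actors at the points of a spline.
; Its Spawn event loops over every spline point and spawns the class at the matching index of the PointClass array at that point's world location.
; Each actor gets zero rotation and unit scale, with the spawner as owner and the event's Instigator passed through.
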(event `Spawn`
  (params (Instigator :type "Pawn Object Reference"))
  (for _index (range (`SplineComponent.GetNumberOfSplinePoints` (`self.Spline`)))
    (`|SpawnActorFromClass` (`|GetArrayItem` (`self.PointClass`) _index) (`KismetMathLibrary.MakeTransform` (`SplineComponent.GetLocationAtSplinePoint` (`self.Spline`) _index "World")) "Undefined" "MultiplyWithRoot" self Instigator)))

(fn `UserConstructionScript`)