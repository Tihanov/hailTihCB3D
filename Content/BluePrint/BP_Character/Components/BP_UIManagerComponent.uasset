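; BP_UIManagerComponent is a component on a PlayerController that owns the main UI screens and switches between them.
; On BeginPlay it creates the default UI, inventory, dialogue and quest menu widgets, displaying only the default one.
; OpenUiAndClosePrevious maps a UI enum to its cached widget, adds it to the viewport and removes the previous one.
; The same call sets game pause and cursor visibility, choosing Game-and-UI input when paused and game-only otherwise.
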(event `self.ReceiveBeginPlay`
  ;[1 1 1] Init
  (`|ExecutionSequence`
    (:`then_0`
      (bind _returnvalue (`|CreateWidget` "/Game/UI/WB_UI.WB_UI_C"))
      (bind _output_get (set `self.DefaultUI` _returnvalue))
      (`/Game/UI/WB_UI.Init` _output_get)
      (`UserWidget.AddToViewport` _output_get 0))
    (:`then_1`
      (bind _returnvalue_2 (`|CreateWidget` "/Game/UI/Inventory/WB_Inventory.WB_Inventory_C"))
      (bind _output_get_2 (set `self.InventoryWidget` _returnvalue_2))
      (`/Game/UI/Inventory/WB_Inventory.Init` _output_get_2))
    (:`then_2`
      (bind _returnvalue_3 (`|CreateWidget` "/Game/UI/Dev/WB_DialogueUI.WB_DialogueUI_C"))
      (set `self.DialogueWidget` _returnvalue_3))
    (:`then_3`
      (bind _returnvalue_4 (`|CreateWidget` "/Game/UI/Dev/WB_QuestMenu.WB_QuestMenu_C"))
      (bind _output_get_3 (set `self.QuestWidget` _returnvalue_4))
      (`/Game/UI/Dev/WB_QuestMenu.Init` _output_get_3))))

(fn `GetCurrentUI`
  (returns (UI :type "UserWidget Object Reference"))
  (return (`self.UIEnumToUserWidget` (`self.WhatUI?`))))

(fn `OpenUiAndClosePrevious`
  (params (ToOpen :type "/Game/BluePrint/BP_Character/UIEnum Enum" :default "NewEnumerator1") (`SetPause?` :type Boolean) (`Show Mouse?` :type Boolean))
  (returns (UI :type "UserWidget Object Reference"))
  (bind _ui (`self.UIEnumToUserWidget` ToOpen))
  (bind _ui_2 (`self.GetCurrentUI`))
  (`GameplayStatics.SetGamePaused` `SetPause?`)
  (bind _asplayer_controller (cast `PlayerController` (`self.GetOwner`)))
  (set `PlayerController.bShowMouseCursor` `Show Mouse?` _asplayer_controller)
  (`UserWidget.AddToViewport` _ui 0)
  (if `SetPause?`
    (`WidgetBlueprintLibrary.SetInputMode_GameAndUIEx` _asplayer_controller _ui "DoNotLock" `Show Mouse?`)
    (else
      (`WidgetBlueprintLibrary.SetInputMode_GameOnly` _asplayer_controller)))
  (`Widget.RemoveFromParent` _ui_2)
  (set `self.WhatUI?` ToOpen)
  (return _ui_2))

(fn `UIEnumToUserWidget`
  (params (`UI Enum` :type "/Game/BluePrint/BP_Character/UIEnum Enum" :default "NewEnumerator1"))
  (returns (UI :type "UserWidget Object Reference"))
  (return (select `/Game/BluePrint/BP_Character/UIEnum` `UI Enum` :`NewEnumerator1` (`self.DefaultUI`) :`NewEnumerator0` (`self.InventoryWidget`) :`NewEnumerator3` (`self.DialogueWidget`) :`NewEnumerator4` (`self.QuestWidget`) :!type "UserWidget Object Reference")))