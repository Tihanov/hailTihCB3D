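; Player character with camera-relative movement, an aim mode, and weapon handling driven by its InventoryManager.
; Aiming requires a weapon in the equipped slot and swaps cameras, walk speed, rotation mode, UI and pistol montage.
; Equip delegates spawn the data-table weapon onto the hand socket or destroy it on unequip.
; Shooting while aiming is forwarded to that weapon through an interface message.
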(event `self.ReceiveBeginPlay`
  (`ActorComponent.SetActive` (`self.AimCamera`) false false)
  (set `CharacterMovementComponent.MaxWalkSpeed` (`self.DefaultSpeed`) (`self.CharacterMovement`)))

(event `InputAxis|MoveForward`
  (params (AxisValue :type "Float (single-precision)"))
  (bind _returnvalue (`KismetMathLibrary.Normal` (`KismetMathLibrary.MakeVector` (.x (`SceneComponent.GetForwardVector` (`self.AimCamera`))) (.y (`SceneComponent.GetForwardVector` (`self.AimCamera`))))))
  (bind _returnvalue_2 (`KismetMathLibrary.Normal` (`KismetMathLibrary.MakeVector` (.x (`SceneComponent.GetForwardVector` (`self.Camera`))) (.y (`SceneComponent.GetForwardVector` (`self.Camera`))))))
  ;[1 1 1] Move Forward
  (if (not (`self.IsInAim?`))
    ;;[1 1 1] NoAimForwardMove
    (`self.AddMovementInput` (select `bool` (== _returnvalue_2 (0.0 0.0 0.0)) :`false` _returnvalue_2 :`true` (`SceneComponent.GetUpVector` (`self.Camera`))) AxisValue)
    (else
      ;;[1 1 1] InAimForwardMove
      (`self.AddMovementInput` (select `bool` (== _returnvalue (0.0 0.0 0.0)) :`false` _returnvalue :`true` (`SceneComponent.GetUpVector` (`self.Camera`))) AxisValue))))

(event `Aim`
  (bind _isinaim_ (`self.IsInAim?`))
  ;[1 1 1] Aim/Unaim
  (if (`InventoryComponent.GetEquippedWeaponIndex` (`self.InventoryManager`)) :!label _label
    (`/Game/BluePrint/BP_Character/Components/BP_UIManagerComponent.OpenUiAndClosePrevious` (`self.GetComponentByClass` (`self.GetController`) "/Game/BluePrint/BP_Character/Components/BP_UIManagerComponent.BP_UIManagerComponent_C") "NewEnumerator6" false false)
    (`self.PlayAnimMontage` "/Game/BluePrint/BP_Character/Character/Animation/Aim/Pistol_Idle_Montage.Pistol_Idle_Montage")
    (`SceneComponent.K2_SetWorldRotation` (`self.CapsuleComponent`) (`KismetMathLibrary.MakeRotator` 0.0 0.0 (.yaw (`SceneComponent.K2_GetComponentRotation` (`self.Camera`)))) false false)
    (set `CharacterMovementComponent.MaxWalkSpeed` (`self.InAimSpeed`) (`self.CharacterMovement`))
    (set `self.IsInAim?` true)
    (`ActorComponent.SetActive` (`self.AimCamera`) _isinaim_ false :!label _label_2)
    (`ActorComponent.SetActive` (`self.Camera`) (not _isinaim_) false)
    (set `CharacterMovementComponent.bOrientRotationToMovement` (not _isinaim_) (`self.CharacterMovement`))
    (set `self.bUseControllerRotationYaw` _isinaim_)))

(event `Key|RightMouseButton`
  (params (Key :type "Key Structure"))
  ;[1 1 1] Aim/Unaim
  (:`Pressed`
    (goto _label))
  (:`Released`
    (`/Game/BluePrint/BP_Character/Components/BP_UIManagerComponent.OpenUiAndClosePrevious` (`self.GetComponentByClass` (`self.GetController`) "/Game/BluePrint/BP_Character/Components/BP_UIManagerComponent.BP_UIManagerComponent_C") "NewEnumerator1" false false :!label _label_3)
    (`self.StopAnimMontage` "/Game/BluePrint/BP_Character/Character/Animation/Aim/Pistol_Idle_Montage.Pistol_Idle_Montage")
    (set `CharacterMovementComponent.MaxWalkSpeed` (`self.DefaultSpeed`) (`self.CharacterMovement`))
    (set `self.IsInAim?` false)
    (goto _label_2)))

(event `Unaim`
  ;[1 1 1] Aim/Unaim
  (goto _label_3))

(event `InputAxis|MoveRight`
  (params (AxisValue :type "Float (single-precision)"))
  ;[1 1 1] Move Right(In or not in aim)
  (`self.AddMovementInput` (`SceneComponent.GetRightVector` (select `bool` (`self.IsInAim?`) :`false` (`self.Camera`) :`true` (`self.AimCamera`) :!type "SceneComponent Object Reference")) AxisValue))

(event `InputAxis|Turn`
  (params (AxisValue :type "Float (single-precision)"))
  ;[1 1 1] PC_Turn and Look Input
  (`self.AddControllerYawInput` AxisValue))

(event `InputAxis|LookUp`
  (params (AxisValue :type "Float (single-precision)"))
  ;[1 1 1] PC_Turn and Look Input
  (`self.AddControllerPitchInput` AxisValue))

(event `self.InventoryManager.OnEquipWeaponFromSlotDelegate`
  (params (EquippedWeaponIndex :type Integer) (SlotIndex :type Integer) (Options :type "InvItemArray Structure"))
  (bind _inhanditem (`self.InHandItem`))
  ;[1 1 1] OnSetItemInHand
  (`/Engine/EditorBlueprintResources/StandardMacros.IsValid` _inhanditem
    (:`Is Valid`
      (`self.K2_DestroyActor` _inhanditem))
    (:`Is Not Valid`
      _))
  (bind _returnvalue (`|GetDataTableRow` (`InventoryComponent.InvDataTable` (`self.InventoryManager`)) Options_RowName)
    (:`then`
      (bind (_displayname _description _type _mesh _ico _weightkg _buyprice _sellprice _maxstackcount _other) (break `InvItemDataTable` _returnvalue))
      (bind ((`Class` _class) (`Scale` _scale) (`WeaponItemSettings` _weaponitemsettings)) (break `InvItemDataTableOptional` _other))
      (`Log.Warning_WithCondition` "Equiped item is not a weapon" (not (and (`|EnumEquality` _type "Weapon") (break `InvWeaponItemSettings` _weaponitemsettings))) "LO_Both")
      (bind _returnvalue_2 (`|SpawnActorFromClass` _class (`KismetMathLibrary.MakeTransform` (0.0 0.0 0.0) (struct) _scale) "AlwaysSpawn" "OverrideRootScale" null self))
      (`Log.Error_WithCondition` "Equiped item do not implement inv weapon interface" (not (`KismetSystemLibrary.DoesImplementInterface` _returnvalue_2 "/Script/AndroidTest.InvWeaponItemInterface")) "LO_Both")
      (`InventoryItemBaseActor.Init` _returnvalue_2 (make `InventoryItemInitStruct` Options_RowName (`InventoryComponent.InvDataTable` (`self.InventoryManager`)) Options_Count))
      (message `InvWeaponItemInterface.InitAsEquippedWeapon` _returnvalue_2 _returnvalue)
      (`self.K2_AttachToComponent` _returnvalue_2 (`self.Mesh`) "PistolSocket" "SnapToTarget" "SnapToTarget" "KeepRelative" true)
      (set `self.InHandItem` _returnvalue_2))))

(event `self.InventoryManager.OnUnequipWeaponDelegate`
  (bind _inhanditem (`self.InHandItem`))
  ;[1 1 1] UnequipItem
  (`/Engine/EditorBlueprintResources/StandardMacros.IsValid` _inhanditem
    (:`Is Valid`
      (`self.K2_DestroyActor` _inhanditem))
    (:`Is Not Valid`
      _))
  (set `self.InHandItem` null))

(event `Key|LeftMouseButton`
  (params (Key :type "Key Structure"))
  (:`Pressed`
    (if (`self.IsInAim?`) :!label _label_4
      (`/Engine/EditorBlueprintResources/StandardMacros.IsValid` (`self.InHandItem`)
        (:`Is Valid`
          (message `InvWeaponItemInterface.Shoot` (`self.InHandItem`) self))
        (:`Is Not Valid`
          (`Log.Warning` "Item is not valid" "LO_Viewport"))))))

(event `Shoot`
  (goto _label_4))

(fn `UserConstructionScript`)