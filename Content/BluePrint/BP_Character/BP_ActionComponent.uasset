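; Action component on a player controller that tracks nearby inventory item actors the player can select.
; Tick, throttled by a short Delay, sphere-traces forward from the controlled pawn, stores InventoryItemBaseActor hits and prints their count.
; The selection index is clamped to the list, stepped by NextEvent and PrevEvent, and resolved to an item by GetCurrentEvent.
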(event `self.ReceiveTick`
  (params (DeltaSeconds :type "Float (single-precision)"))
  (bind _returnvalue (`KismetArrayLibrary.Array_Length` (`self.EventsArray`)))
  (bind _returnvalue_2 (`Controller.K2_GetPawn` (cast `PlayerController` (`self.GetOwner`) :!pure true)))
  (if (`KismetMathLibrary.Conv_IntToBool` _returnvalue)
    (if (>= (`self.EventIndex`) _returnvalue)
      (set `self.EventIndex` (- _returnvalue 1)))
    (else
      (set `self.EventIndex` 0)))
  (`KismetSystemLibrary.Delay` 0.1)
  (bind _array (`self.ScanForEvents` "/Script/AndroidTest.InventoryItemBaseActor" (`Actor.K2_GetActorLocation` _returnvalue_2) (`Actor.GetActorForwardVector` _returnvalue_2) (`self.ScanRadious`) (`|MakeArray` _returnvalue_2 :!type "Actor Object Reference") (`self.UseDebug`)))
  (bind _output_get (set `self.EventsArray` _array))
  (`KismetSystemLibrary.PrintString` (`KismetStringLibrary.Conv_IntToString` (`KismetArrayLibrary.Array_Length` _output_get))))

(fn `GetCurrentEvent`
  (returns (NewParam :type "InventoryItemBaseActor Object Reference"))
  (bind _eventsarray (`self.EventsArray`))
  (if (`KismetMathLibrary.Conv_IntToBool` (`KismetArrayLibrary.Array_Length` _eventsarray))
    (return (cast `InventoryItemBaseActor` (`|GetArrayItem` _eventsarray (`self.EventIndex`)) :!pure true))
    (else
      (return null))))

(fn `Next Event`
  (if (< (`self.EventIndex`) (- (`KismetArrayLibrary.Array_Length` (`self.EventsArray`)) 1))
    (`/Engine/EditorBlueprintResources/StandardMacros.IncrementInt` (`self.EventIndex`))))

(fn `Prev Event`
  (if (!= (`self.EventIndex`) 0)
    (`/Engine/EditorBlueprintResources/StandardMacros.DecrementInt` (`self.EventIndex`))))

(fn `ScanForEvents`
  (params (Class :type "Actor Class Reference") (Location :type "Vector Structure") (Derection :type "Vector Structure") (Radious :type "Float (double-precision)") (ActorsToIgnore :type "Array of Actor Object Reference") (`UseDebug?` :type Boolean))
  (returns (Array :type "Array of Actor Object Reference"))
  (locals (EventsArrayLocal :type "Array of Actor Object Reference"))
  (bind (_outhits _returnvalue) (`KismetSystemLibrary.SphereTraceMulti` Location (+ Location (* Derection Radious)) 100.0 "TraceTypeQuery1" false ActorsToIgnore (select `bool` `UseDebug?` :`true` "ForOneFrame" :!type "EDrawDebugTrace Enum")))
  (if _returnvalue
    (for _array_element _outhits
      (bind (_bblockinghit _binitialoverlap _time _distance _location _impactpoint _normal _impactnormal _physmat _hitactor) (`GameplayStatics.BreakHitResult` _array_element))
      (if (`KismetMathLibrary.ClassIsChildOf` (`GameplayStatics.GetObjectClass` _hitactor) Class)
        (`KismetArrayLibrary.Array_Add` (`local.EventsArrayLocal`) _hitactor))))
  (return (`local.EventsArrayLocal`)))