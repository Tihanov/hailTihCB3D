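; Quest task that completes when the player starts a dialogue that includes a specified NPC.
; Init sets the soft-referenced NPC's quest status to "have questions" and binds to the player character's dialogue-about-to-start delegate, warning if no NPC is set.
; When that NPC is among the participants, the task marks itself complete, fires its done delegate and clears the NPC's status.
; Its display name is Russian "Talk to" text plus the NPC's dialogue name.
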(event `self.Init`
  (params (PlayerController :type "PlayerController Object Reference"))
  (if (`KismetSystemLibrary.IsValidSoftObjectReference` (`self.Npc`))
    (bind _aspc_character (cast `/Game/BluePrint/BP_Character/PC_Character` PlayerController))
    (add `MainPlayerController.OnDialogueAboutToStartDelegate` _aspc_character (delegate `OnDialogueAboutToStartDelegate_Event`))
    (set `NpcCharacter.QuestStatus` "QSHaveQuestions" (`|ConvertAsset` (`self.Npc`)))
    (else
      (`Log.Warning` "Установите объект, с которим будеде говорить" "LO_Both"))))

(event `OnDialogueAboutToStartDelegate_Event`
  (params (PlayerController :type "PlayerController Object Reference") (Participants :type "ProxyStructArrayOfParticipants Structure"))
  (for _array_element Participants_Participants
    (if (and (== _array_element (`|ConvertAsset` (`self.Npc`))) (not (`self.IsComplete?`)))
      (set `self.IsComplete?` true)
      (`self.OnTaskDoneDelegate` self)
      (set `NpcCharacter.QuestStatus` "QSNone" (`|ConvertAsset` (`self.Npc`))))))

(fn `GetDisplayName`
  (returns (ReturnValue :type Text))
  (return (`|FormatText` "{Task} {Name}" (`|FormatText` "Поговорите с") (`NpcCharacter.DlgDisplayName` (`|ConvertAsset` (`self.Npc`))))))

(fn `IsDone`
  (returns (ReturnValue :type Boolean))
  (return (`self.IsComplete?`)))