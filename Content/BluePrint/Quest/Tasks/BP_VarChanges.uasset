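; BP_VarChanges is a quest task that completes when a quest variable holds an expected value.
; On Init it gets the player controller's QuestManagerComponent and signals task done at once if the variable already matches.
; Otherwise it binds to the manager's variable-changed delegate and signals done on a matching change, logging warnings if controller or manager is missing.
; It exposes Title as display name and an IsDone flag, which these graphs never set.
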(event `self.BP_Init`
  (params (PlayerController :type "PlayerController Object Reference"))
  (bind _returnvalue (`Actor.GetComponentByClass` PlayerController "/Script/AndroidTest.QuestManagerComponent"))
  (bind (_outexist _returnvalue_2) (`QuestManagerComponent.GetQuestVariable` _returnvalue (`self.Quest Asset`) (`self.VarName`)))
  (`/Engine/EditorBlueprintResources/StandardMacros.IsValid` PlayerController
    (:`Is Valid`
      (`/Engine/EditorBlueprintResources/StandardMacros.IsValid` _returnvalue
        (:`Is Valid`
          (if (and _outexist (== _returnvalue_2 (`self.ExpectedValue`)))
            (`self.OnTaskDoneDelegate` self self)
            (else
              (add `QuestManagerComponent.OnQuestVariableChangedDelegate` _returnvalue (delegate `OnQuestVariableChangedDelegate_Event`)))))
        (:`Is Not Valid`
          (`Log.Warning` "BP_VarChanges: QuestManagerComponent == nullptr" "LO_Both" false 5.0 "None" null))))
    (:`Is Not Valid`
      (`Log.Warning` "BP_VarChanges: PlayerController == nullptr" "LO_Both" false 5.0 "None" null))))

(event `OnQuestVariableChangedDelegate_Event`
  (params (QuestManagerComponent :type "QuestManagerComponent Object Reference") (Quest :type "QuestAsset Object Reference") (VarName :type Name) (Value :type Integer))
  (if (and (== (`self.Quest Asset`) Quest) (== (`self.VarName`) VarName) (== (`self.ExpectedValue`) Value))
    (`self.OnTaskDoneDelegate` self self)))

(fn `GetDisplayName`
  (returns (ReturnValue :type Text))
  (return (`self.Title`)))

(fn `IsDone`
  (returns (ReturnValue :type Boolean))
  (return (`self.IsDone?`)))