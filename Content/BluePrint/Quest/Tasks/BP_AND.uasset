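; BP_AND is a composite quest task that groups a list of child Tasks under an AND label.
; GetDisplayName loops over the children and chains their display names into one text separated by "AND".
; IsDone returns a stored IsDone variable without checking the children, and the Init event is empty.
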(event `self.BP_Init`
  (params (PlayerController :type "PlayerController Object Reference")))

(fn `GetDisplayName`
  (returns (ReturnValue :type Text))
  (locals (ToRet :type Text))
  (for (_array_element _array_index) (`self.Tasks`)
    (if (== _array_index 0)
      (bind _returnvalue (`self.GetDisplayName` _array_element))
      (set `local.ToRet` _returnvalue)
      (else
        (set `local.ToRet` (`|FormatText` "{0} \nAND \n{1}" (`local.ToRet`) _returnvalue)))))
  (return (`local.ToRet`)))

(fn `IsDone`
  (returns (ReturnValue :type Boolean))
  (return (`self.bIsDone`)))