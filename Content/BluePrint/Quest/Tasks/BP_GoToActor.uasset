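; Quest task that completes when the player reaches a target actor, set as a soft reference.
; On Init it binds to the controlled pawn's begin-overlap and hit events, or logs a warning if the target reference is invalid.
; Either event marks the task complete when the other actor is the target, then fires the task-done delegate once.
; Its display name is a Ukrainian "go to" prompt plus the target's name.
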(event `self.Init`
  (params (PlayerController :type "PlayerController Object Reference"))
  (bind _returnvalue (`Controller.K2_GetPawn` PlayerController))
  (if (`KismetSystemLibrary.IsValidSoftObjectReference` (`self.Actor`))
    (add `Actor.OnActorBeginOverlap` _returnvalue (delegate `OnActorBeginOverlap_Event_0`))
    (add `Actor.OnActorHit` _returnvalue (delegate `CustomEvent_0`))
    (else
      (`Log.Warning` "Встанови обєкт, то якого будеш йти" "LO_Both"))))

(event `OnActorBeginOverlap_Event_0`
  (params (OverlappedActor :type "Actor Object Reference") (OtherActor :type "Actor Object Reference"))
  (if (not (`self.IsComplete?`))
    (bind _output_get (set `self.IsComplete?` (== (`|ConvertAsset` (`self.Actor`)) OtherActor)))
    (if _output_get
      (`self.OnTaskDoneDelegate` self :!label _label))))

(event `CustomEvent_0`
  (params (SelfActor :type "Actor Object Reference") (OtherActor :type "Actor Object Reference") (NormalImpulse :type "Vector Structure") (Hit :type "HitResult Structure (by ref)"))
  (if (not (`self.IsComplete?`))
    (bind _output_get (set `self.IsComplete?` (== (`|ConvertAsset` (`self.Actor`)) OtherActor)))
    (if _output_get
      (goto _label))))

(fn `GetDisplayName`
  (returns (ReturnValue :type Text))
  (return (`KismetTextLibrary.Conv_StringToText` (`KismetStringLibrary.Concat_StrStr` "Дойди до " (`KismetSystemLibrary.GetDisplayName` (`|ConvertAsset` (`self.Actor`)))))))

(fn `IsDone`
  (returns (ReturnValue :type Boolean))
  (return (`self.IsComplete?`)))