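; BP_SetDialogueForNpc is a quest follow-up action that assigns a dialogue to an NPC.
; Its Do event resolves the soft Npc reference and calls SetDialogue with the Dialogue and QuestStatus variables.
; If Dialogue or the Npc reference is not valid, it logs a warning that both must be set.
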(event `self.Do`
  (params (QuestManagerComponent :type "QuestManagerComponent Object Reference"))
  (if (and (`KismetSystemLibrary.IsValid` (`self.Dialogue`)) (`KismetSystemLibrary.IsValidSoftObjectReference` (`self.Npc`)))
    (`NpcBaseCharacter.SetDialogue` (`|ConvertAsset` (`self.Npc`)) (`self.Dialogue`) (`self.QuestStatus`))
    (else
      (`Log.Warning` "установите Npc и Dialogue в BP_SetDialogueForNpc" "LO_Both" false 5.0 "None" null))))