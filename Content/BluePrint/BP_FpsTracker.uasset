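; BP_FpsTracker is a helper Blueprint that measures frame rate by counting updates per second.
; Its Update function accumulates the passed-in delta time and increments a tick counter on each call.
; Once a full second has accumulated, it resets both values and returns the count with an update flag; otherwise it returns false and zero.
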(fn `Update`
  (params (DeltaTime :type "Float (double-precision)"))
  (returns (`Updates?` :type Boolean) (TickCount :type Integer))
  (locals (TempTick :type Integer))
  (set `self.CurrentTimeRemain` (+ DeltaTime (`self.CurrentTimeRemain`)))
  (`/Engine/EditorBlueprintResources/StandardMacros.IncrementInt` (`self.TickCount`)
    (:`  `
      (if (>= (`self.CurrentTimeRemain`) 1.0)
        (set `self.CurrentTimeRemain` 0.0)
        (bind _output_get (set `local.TempTick` (`self.TickCount`)))
        (set `self.TickCount` 0)
        (return true _output_get)
        (else
          (return false 0))))))

(fn `UserConstructionScript`)