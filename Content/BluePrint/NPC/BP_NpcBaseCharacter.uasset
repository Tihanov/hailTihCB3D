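; BP_NpcBaseCharacter is a base NPC character Blueprint that stubs out a dialogue participant interface.
; It declares hooks for dialogue events, condition checks, participant icon and gender, and getting or modifying name, int, float and bool values.
; All hooks return defaults such as false, zero, None or Masculine, and BeginPlay and the construction script are empty.
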(fn `CheckCondition`
  (params (Context :type "DlgContext Object Reference") (ConditionName :type Name :default "None"))
  (returns (ReturnValue :type Boolean))
  (return false))

(fn `GetBoolValue`
  (params (ValueName :type Name :default "None"))
  (returns (ReturnValue :type Boolean))
  (return false))

(fn `GetFloatValue`
  (params (ValueName :type Name :default "None"))
  (returns (ReturnValue :type "Float (double-precision)"))
  (return 0.0))

(fn `GetIntValue`
  (params (ValueName :type Name :default "None"))
  (returns (ReturnValue :type Integer))
  (return 0))

(fn `GetNameValue`
  (params (ValueName :type Name :default "None"))
  (returns (ReturnValue :type Name))
  (return "None"))

(fn `GetParticipantGender`
  (returns (ReturnValue :type "ETextGender Enum"))
  (return "Masculine"))

(fn `GetParticipantIcon`
  (params (ActiveSpeaker :type Name :default "None") (ActiveSpeakerState :type Name :default "None"))
  (returns (ReturnValue :type "Texture2D Object Reference"))
  (return null))

(fn `ModifyBoolValue`
  (params (ValueName :type Name :default "None") (bNewValue :type Boolean :default false))
  (returns (ReturnValue :type Boolean))
  (return false))

(fn `ModifyFloatValue`
  (params (ValueName :type Name :default "None") (bDelta :type Boolean :default false) (Value :type "Float (double-precision)" :default 0.0))
  (returns (ReturnValue :type Boolean))
  (return false))

(fn `ModifyIntValue`
  (params (ValueName :type Name :default "None") (bDelta :type Boolean :default false) (Value :type Integer :default 0))
  (returns (ReturnValue :type Boolean))
  (return false))

(fn `ModifyNameValue`
  (params (ValueName :type Name :default "None") (NameValue :type Name :default "None"))
  (returns (ReturnValue :type Boolean))
  (return false))

(fn `OnDialogueEvent`
  (params (Context :type "DlgContext Object Reference") (EventName :type Name :default "None"))
  (returns (ReturnValue :type Boolean))
  (return false))

(fn `UserConstructionScript`)