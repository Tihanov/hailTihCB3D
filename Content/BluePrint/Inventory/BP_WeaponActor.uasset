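; BP_WeaponActor is an inventory weapon actor that converts from a pickup into an equipped gun able to fire line traces.
; InitasEquippedWeapon copies magazine capacity and range from item settings, disables physics, collision, name text and pickup, or warns if the mesh lacks a ShootFrom socket.
; Shoot traces from that socket along the shooter pawn's aim, currently only drawing and printing debug output, with no damage or ammo use.
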(event `InvWeaponItemInterface.Shoot`
  (params (CausedBy :type "Actor Object Reference"))
  (bind _returnvalue (`SceneComponent.GetSocketLocation` (`self.RootMeshComponent`) "ShootFrom"))
  (bind _aspawn (cast `Pawn` CausedBy))
  (`KismetSystemLibrary.PrintString` "Hello")
  (bind _outhit (`KismetSystemLibrary.LineTraceSingle` _returnvalue (+ _returnvalue (* (`KismetMathLibrary.GetForwardVector` (`Pawn.GetBaseAimRotation` _aspawn)) (`self.ShotRange`))) "TraceTypeQuery1" false (`|MakeArray` CausedBy) "Persistent"))
  (`KismetSystemLibrary.PrintString` (`KismetSystemLibrary.GetDisplayName` (`.HitActor` (`GameplayStatics.BreakHitResult` _outhit)))))

(event `InvWeaponItemInterface.InitAsEquippedWeapon`
  (params (Options :type "InvItemDataTable Structure"))
  (bind _rootmeshcomponent (`self.RootMeshComponent`))
  (bind (_weaponitemsettings_bisweapon _weaponitemsettings_magazinecapacity _weaponitemsettings_shotrange) (break `InvWeaponItemSettings` (break `InvItemDataTableOptional` (`.Other` (break `InvItemDataTable` Options)))))
  (if (`SceneComponent.DoesSocketExist` (`self.RootMeshComponent`) "ShootFrom")
    (`|ExecutionSequence`
      (:`then_0`
        (set `self.MagazineCapacity` _weaponitemsettings_magazinecapacity))
      (:`then_1`
        (set `self.ShotRange` _weaponitemsettings_shotrange))
      (:`then_2`
        (`PrimitiveComponent.SetSimulatePhysics` _rootmeshcomponent false))
      (:`then_3`
        (`PrimitiveComponent.SetCollisionEnabled` _rootmeshcomponent "NoCollision"))
      (:`then_4`
        (`SceneComponent.SetHiddenInGame` (`self.DisplayNameText`) true false))
      (:`then_5`
        (set `self.bCanBePickUpped` false)))
    (else
      (`Log.Warning` "Add ShootFrom socket to Weapon Mesh" "LO_Both"))))

(fn `UserConstructionScript`
  (`parent.UserConstructionScript`))