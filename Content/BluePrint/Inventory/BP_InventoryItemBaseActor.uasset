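; Base actor for an inventory item in the world, showing a floating label with its name and count.
; The construction script initializes it from DT_Items by RowName, while a first-Tick setup positions the label atop the mesh, sets item collision and reads the display name from the GameState's inventory table.
; Each Tick refreshes the text when the count changes, turns it toward the player camera and shows it only within render range.
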(event `self.ReceiveTick`
  (params (DeltaSeconds :type "Float (single-precision)"))
  (bind _returnvalue (`GameplayStatics.GetPlayerPawn` 0))
  (bind _displaynametext (`self.DisplayNameText`))
  (bind _returnvalue_2 (`SceneComponent.GetRelativeTransform` _displaynametext))
  (bind _returnvalue_3 (`SceneComponent.K2_GetComponentLocation` (`self.DisplayNameText`)))
  (bind _returnvalue_4 (`self.GetComponentByClass` _returnvalue "/Script/Engine.CameraComponent"))
  (`|ExecutionSequence`
    (:`then_0`
      (`/Engine/EditorBlueprintResources/StandardMacros.DoOnce` false
        (:`Completed`
          (`SceneComponent.SetAbsolute` (`self.DisplayNameTextPivot`) false true false)
          (`SceneComponent.SetAbsolute` _displaynametext false false true)
          (`SceneComponent.SetRelativeScale3D` _displaynametext (1.0 1.0 1.0))
          (`SceneComponent.K2_SetRelativeLocation` _displaynametext (`KismetMathLibrary.MakeVector` (.x (.location _returnvalue_2)) (.y (.location _returnvalue_2)) (.z (`.Max` (`StaticMeshComponent.GetLocalBounds` (`self.RootMeshComponent`))))) false true)
          (`PrimitiveComponent.SetCollisionProfileName` (`self.RootMeshComponent`) "InventoryItem" true)
          (bind _returnvalue_5 (`|GetDataTableRow` (`MainGameState.InventoryDataTable` (cast `MainGameState` (`GameplayStatics.GetGameState`) :!pure true)) (`self.RowName`))
            (:`then`
              (set `self.Display Name` (`.DisplayName` (break `InvItemDataTable` _returnvalue_5))))))))
    (:`then_1`
      (if (!= (`self.CountOfTemp`) (`self.CountOf`))
        (`TextRenderComponent.K2_SetText` (`self.DisplayNameText`) (`KismetTextLibrary.Conv_StringToText` (`KismetStringLibrary.Concat_StrStr` (`KismetTextLibrary.Conv_TextToString` (`self.Display Name`)) " x" (`KismetStringLibrary.Conv_IntToString` (`self.CountOf`)))))
        (set `self.CountOfTemp` (`self.CountOf`))))
    (:`then_2`
      (`/Engine/EditorBlueprintResources/StandardMacros.IsValid` _returnvalue_4
        (:`Is Valid`
          (`SceneComponent.K2_SetWorldRotation` (`self.DisplayNameText`) (`KismetMathLibrary.FindLookAtRotation` _returnvalue_3 (`SceneComponent.K2_GetComponentLocation` _returnvalue_4)) false false))))
    (:`then_3`
      (`SceneComponent.SetVisibility` (`self.DisplayNameText`) (< (`KismetMathLibrary.Vector_Distance` _returnvalue_3 (`self.K2_GetActorLocation` _returnvalue)) (`self.DisplayNameTextRenderRange`)) false))))

(fn `UserConstructionScript`
  (`/Game/BluePrint/Utilities/MacroUtil.DefaultInventoryInit` self "/Game/BluePrint/Inventory/DT_Items.DT_Items" (`self.RowName`)))