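; Custom EQS generator that produces candidate cover points for AI around each context location.
; It spaces trace starts evenly on a horizontal ring of configurable radius and count, then line-traces inward to the context location.
; Each hit yields a point pushed off the surface normal plus an offset, on the obstacle side facing away from the context.
; Actor-based generation is empty, and an uncalled GeneratePointFromLocation variant uses a fixed upward offset.
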(fn `DoItemGeneration`
  (params (ContextLocations :type "Array of Vector Structure (by ref)"))
  (for _array_element ContextLocations
    (for _index (range (`self.CountOfPoint`))
      (bind (_outhit _returnvalue) (`KismetSystemLibrary.LineTraceSingle` (+ (* (`KismetMathLibrary.GreaterGreater_VectorRotator` (1.0 0.0 0.0) (`KismetMathLibrary.MakeRotator` 0.0 0.0 (* (/ 360 (`self.CountOfPoint`)) _index))) (`self.Radius`)) _array_element) _array_element (cast `ETraceTypeQuery` 2)))
      (if _returnvalue
        (bind (_bblockinghit _binitialoverlap _time _distance _location _impactpoint _normal _impactnormal) (`GameplayStatics.BreakHitResult` _outhit))
        (`self.AddGeneratedVector` (+ _impactpoint (`self.PointOffset`) (* _impactnormal 50.0))))))
  (return))

(fn `DoItemGenerationFromActors`
  (params (ContextActors :type "Array of Actor Object Reference (by ref)"))
  (return))

(fn `GeneratePointFromLocation`
  (params (Location :type "Vector Structure"))
  (for _index (range (`self.CountOfPoint`))
    (bind (_outhit _returnvalue) (`KismetSystemLibrary.LineTraceSingle` (+ (* (`KismetMathLibrary.GreaterGreater_VectorRotator` (1.0 0.0 0.0) (`KismetMathLibrary.MakeRotator` 0.0 0.0 (* (/ 360 (`self.CountOfPoint`)) _index))) (`self.Radius`)) Location) Location (cast `ETraceTypeQuery` 2)))
    (if _returnvalue
      (`self.AddGeneratedVector` (+ (`.ImpactPoint` (`GameplayStatics.BreakHitResult` _outhit)) (0.0 0.0 200.0))))))