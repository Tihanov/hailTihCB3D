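; Dialogue condition that checks whether a participant is currently on a specific part of a given quest.
; It casts the participant to Actor, reads the current part of the configured quest from its QuestManagerComponent, and compares that part's Id to QuestPartId.
; A non-Actor participant or a missing current part logs a warning instead of performing the comparison.
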(fn `IsConditionMet`
  (params (Context :type "DlgContext Object Reference") (Participant :type "Object Object Reference"))
  (returns (ReturnValue :type Boolean))
  (bind _asactor (cast `Actor` Participant)
    (:`then`
      (bind (_exist _returnvalue) (`QuestManagerComponent.GetCurrentPartFromQuest` (`Actor.GetComponentByClass` _asactor "/Script/AndroidTest.QuestManagerComponent") (`self.Quest`)))
      (if _exist
        (return (== (`.Id` (break `QuestPartInfo` _returnvalue)) (`self.QuestPartId`)))
        (else
          (`Log.Warning` "Quest Part with this Id does not exists" "LO_Both"))))
    (:`CastFailed`
      (`Log.Warning` "Participant should be derived from actor" "LO_Both"))))