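; Dialogue condition that passes when the participant has neither taken nor completed a given quest.
; It casts the participant to an Actor, gets its QuestManagerComponent and looks up Quest in both CurrentQuests and CompletedQuests.
; A failed cast or missing component never reaches the check, so no true result is returned in those cases.
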(fn `IsConditionMet`
  (params (Context :type "DlgContext Object Reference") (Participant :type "Object Object Reference"))
  (returns (ReturnValue :type Boolean))
  (bind _asactor (cast `Actor` Participant))
  (bind _returnvalue (`Actor.GetComponentByClass` _asactor "/Script/AndroidTest.QuestManagerComponent"))
  (`/Engine/EditorBlueprintResources/StandardMacros.IsValid` _returnvalue
    (:`Is Valid`
      (return (not (or (`.ReturnValue` (`BlueprintMapLibrary.Map_Find` (`QuestManagerComponent.CurrentQuests` _returnvalue) (`self.Quest`))) (!= (`KismetArrayLibrary.Array_Find` (`QuestManagerComponent.CompletedQuests` _returnvalue) (`self.Quest`)) -1)))))))