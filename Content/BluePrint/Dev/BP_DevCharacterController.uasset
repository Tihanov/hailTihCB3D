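; Player controller for BP_DevCharacter that handles movement, look, item pickup and the inventory screen.
; It creates the HUD and inventory widgets, swapping them, pausing and changing input mode when toggled.
; A camera line trace picks up items into the Inventory component, leaving any leftover count in the world.
; Thrown-out items respawn at the character from their DataTable row's class, and inventory changes refresh the widget's contents and weight.
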(event `InputAxis|MoveForward`
  (params (AxisValue :type "Float (single-precision)"))
  (bind _characterplayer (`self.CharacterPlayer`))
  ;[1 1 1] Moving
  (`Pawn.AddMovementInput` _characterplayer (`self.GetActorForwardVector` _characterplayer) AxisValue false))

(event `InputAxis|MoveRight`
  (params (AxisValue :type "Float (single-precision)"))
  (bind _characterplayer (`self.CharacterPlayer`))
  ;[1 1 1] Moving
  (`Pawn.AddMovementInput` _characterplayer (`self.GetActorRightVector` _characterplayer) AxisValue false))

(event `self.ReceiveBeginPlay`
  (bind _asbp_dev_character (cast `/Game/BluePrint/Dev/BP_DevCharacter` (`self.K2_GetPawn`))
    (:`then`
      (set `self.CharacterPlayer` _asbp_dev_character)
      (`|ExecutionSequence`
        (:`then_0`
          (bind _returnvalue (`|CreateWidget` "/Game/UI/Dev/WB_Inventory.WB_Inventory_C" self))
          (set `self.InventoryWidget` _returnvalue))
        (:`then_1`
          (bind _returnvalue_2 (`|CreateWidget` "/Game/UI/Dev/WB_UI.WB_UI_C" self))
          (bind _output_get (set `self.UIWIdget` _returnvalue_2))
          (`UserWidget.AddToViewport` _output_get 0))))
    (:`CastFailed`
      (`KismetSystemLibrary.PrintString` "ERRORR"))))

(event `InputAxis|LookUp`
  (params (AxisValue :type "Float (single-precision)"))
  ;[1 1 1] Look
  (bind _result (`/Engine/EditorBlueprintResources/StandardMacros.NegateFloat` AxisValue)
    (:`  `
      (`Pawn.AddControllerPitchInput` (`self.CharacterPlayer`) _result))))

(event `InputAxis|LookRight`
  (params (AxisValue :type "Float (single-precision)"))
  ;[1 1 1] Look
  (`Pawn.AddControllerYawInput` (`self.CharacterPlayer`) AxisValue))

(event `Key|E`
  (params (Key :type "Key Structure"))
  (bind _camera (`/Game/BluePrint/Dev/BP_DevCharacter.Camera` (`self.CharacterPlayer`)))
  (bind _returnvalue (`SceneComponent.K2_GetComponentLocation` _camera))
  ;[1 1 1] Inventory
  (:`Pressed`
    (bind (_outhit _returnvalue_2) (`KismetSystemLibrary.LineTraceSingle` _returnvalue (+ _returnvalue (* (`SceneComponent.GetForwardVector` _camera) 1000.0)) "TraceTypeQuery1" false (`|MakeArray` self :!type "Actor Object Reference")))
    (if _returnvalue_2
      (`self.PickUpItem` (cast `InventoryItemBaseActor` (`.HitActor` (`GameplayStatics.BreakHitResult` _outhit)) :!pure true)))))

(event `self.OpenCloseInventory`
  ;[1 1 1] Open Close Inventory
  (if (`self.InInventory?`)
    (`self.CloseInventory`)
    (else
      (`self.OpenInventory`))))

(event `self.OpenInventory`
  ;[1 1 1] Open Close Inventory
  (if (not (`self.InInventory?`))
    (`GameplayStatics.SetGamePaused` true)
    (set `self.bShowMouseCursor` true)
    (`UserWidget.AddToViewport` (`self.InventoryWidget`) 0)
    (`WidgetBlueprintLibrary.SetInputMode_GameAndUIEx` self (`self.InventoryWidget`) "DoNotLock" false)
    (`Widget.RemoveFromParent` (`self.UIWIdget`))
    (set `self.InInventory?` (not (`self.InInventory?`)) :!label _label)))

(event `self.CloseInventory`
  ;[1 1 1] Open Close Inventory
  (if (`self.InInventory?`)
    (`GameplayStatics.SetGamePaused` false)
    (set `self.bShowMouseCursor` false)
    (`Widget.RemoveFromParent` (`self.InventoryWidget`))
    (`WidgetBlueprintLibrary.SetInputMode_GameOnly` self)
    (`UserWidget.AddToViewport` (`self.UIWIdget`) 0)
    (goto _label)))

(event `Key|I` :paused true
  (params (Key :type "Key Structure"))
  ;[1 1 1] Open Close Inventory
  (:`Pressed`
    (`self.OpenCloseInventory`)))

(fn `GetInventoryComponent`
  (returns (ReturnValue :type "InventoryComponent Object Reference"))
  (return (`self.Inventory`)))

(fn `GetWeight`
  (returns (Weight :type "Float (double-precision)") (MaxWeight :type "Float (double-precision)"))
  (bind _inventory (`self.Inventory`))
  (return (`InventoryComponent.Weight` _inventory) (`InventoryComponent.MaxWeight` _inventory)))

(fn `PickUpItem`
  (params (Item :type "InventoryItemBaseActor Object Reference"))
  (returns (ReturnValue :type Boolean))
  (bind _inventory (`self.Inventory`))
  (bind _inventorywidget (`self.InventoryWidget`))
  (bind _inventory_2 (`self.Inventory`))
  (bind _inventorywidget_2 (`self.InventoryWidget`))
  (`/Engine/EditorBlueprintResources/StandardMacros.IsValid` Item
    (:`Is Valid`
      (bind _returnvalue (`InventoryItemBaseActor.PickUp` Item self))
      (bind _returnvalue_2 (`InventoryComponent.AddItem` (`self.Inventory`) _returnvalue (`InventoryItemBaseActor.CountOf` Item)))
      (if (== _returnvalue_2 0)
        (`self.K2_DestroyActor` Item)
        (`/Game/UI/Dev/WB_Inventory.UpdateInventory` _inventorywidget_2)
        (`/Game/UI/Dev/WB_Inventory.SetWeight` _inventorywidget_2 (`InventoryComponent.Weight` _inventory) (`InventoryComponent.MaxWeight` _inventory))
        (return true)
        (elif (== _returnvalue_2 (`InventoryItemBaseActor.CountOf` Item))
          (return false)
          (else
            (set `InventoryItemBaseActor.CountOf` _returnvalue_2 Item)
            (`/Game/UI/Dev/WB_Inventory.UpdateInventory` _inventorywidget)
            (`/Game/UI/Dev/WB_Inventory.SetWeight` _inventorywidget (`InventoryComponent.Weight` _inventory_2) (`InventoryComponent.MaxWeight` _inventory_2))
            (return true)))))))

(fn `ThrowOutItem`
  (params (Index :type Integer) (Count :type Integer))
  (returns (ReturnValue :type Boolean))
  (bind _inventory (`self.Inventory`))
  (bind _inventorywidget (`self.InventoryWidget`))
  (bind (_rowname _returnvalue) (`InventoryComponent.TrashItem` (`self.Inventory`) Index Count))
  (if _returnvalue
    (bind _returnvalue_2 (`|GetDataTableRow` (`InventoryComponent.InvDataTable` (`self.Inventory`)) _rowname)
      (:`then`
        (bind _returnvalue_3 (`|SpawnActorFromClass` (`.Class` (break `InvItemDataTableOptional` (`.Other` (break `InvItemDataTable` _returnvalue_2)))) (`self.GetTransform` (`self.CharacterPlayer`)) "AlwaysSpawn" "OverrideRootScale" null null))
        (`InventoryItemBaseActor.Init` _returnvalue_3 (make `InventoryItemInitStruct` _rowname (`InventoryComponent.InvDataTable` (`self.Inventory`)) Count))
        (`/Game/UI/Dev/WB_Inventory.UpdateInventory` _inventorywidget)
        (`/Game/UI/Dev/WB_Inventory.SetWeight` _inventorywidget (`InventoryComponent.Weight` _inventory) (`InventoryComponent.MaxWeight` _inventory))
        (return true)))
    (else
      (return false))))

(fn `UserConstructionScript`)