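; Dev damage-causer actor that deals damage around its own location, apparently for testing.
; Every tick it runs a zero-length sphere trace for Pawn objects with persistent debug drawing, using its Radius.
; On a hit it applies Damage to the hit actor's instigator controller rather than to the actor itself, or shows a viewport warning if that controller is invalid.
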(event `self.ReceiveTick`
  (params (DeltaSeconds :type "Float (single-precision)"))
  (bind _returnvalue (`self.K2_GetActorLocation`))
  (bind (_outhit _returnvalue_2) (`KismetSystemLibrary.SphereTraceSingleForObjects` :`Start` _returnvalue :`End` _returnvalue :`Radius` (`self.Radius`) :`ObjectTypes` (`|MakeArray` "ObjectTypeQuery3" :!type "EObjectTypeQuery Enum") :`DrawDebugType` "Persistent"))
  (if _returnvalue_2
    (bind _returnvalue_3 (`self.GetInstigatorController` (`.HitActor` (`GameplayStatics.BreakHitResult` _outhit))))
    (`/Engine/EditorBlueprintResources/StandardMacros.IsValid` _returnvalue_3
      (:`Is Valid`
        (`GameplayStatics.ApplyDamage` _returnvalue_3 (`self.Damage`)))
      (:`Is Not Valid`
        (`Log.Warning` "---------------------------------------" "LO_Viewport")))))

(fn `UserConstructionScript`)