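; Candle prop Blueprint with a point light and flame effect that can be switched on or off through an Enabled flag.
; The construction script passes the flag to IsEnabled, which toggles visibility of PointLight and FXCandleLight.
; The same function disables shadow casting on the candle mesh while lit and restores it when unlit.
; BeginPlay sets the point light to a fixed intensity, and Tick is unused.
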(event `self.ReceiveBeginPlay`
  (`LightComponent.SetIntensity` (`self.PointLight`) 20.0))

(fn `isEnabled`
  (params (`Enabled?` :type Boolean))
  (bind _output_get (set `self.Enabled?` `Enabled?`))
  (`SceneComponent.SetVisibility` (`self.PointLight`) _output_get false)
  (`SceneComponent.SetVisibility` (`self.FX_CandleLight`) _output_get false)
  (`PrimitiveComponent.SetCastShadow` (`self.SM_CandleA`) (not _output_get)))

(fn `UserConstructionScript`
  (`self.isEnabled` (`self.Enabled?`)))